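; AIC_Runner is an AI controller that drives a BP_Runner pawn by faking player power input.
; It caches the runner on possess and starts a one-shot timer with a random delay on BeginPlay.
; SimulateInput uses a FlipFlop to alternate left and right power calls on the runner, re-arming the random timer after each press.
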(event Custom|SimulateInput
  (bind _as_bp_runner (Variables|Default|GetAs%20BP%20Runner))
  (Utilities|FlowControl|FlipFlop
    (:A
      (Default|SimulatePowerLeft _as_bp_runner)
      (CallFunction|SimulateInputwithDelay))
    (:B
      (Default|SimulatePowerRight _as_bp_runner)
      (CallFunction|SimulateInputwithDelay))))

(event EventBeginPlay
  (CallFunction|SimulateInputwithDelay))

(event EventPossess
  (params (PossessedPawn :type Pawn%20Object%20Reference))
  (bind _asbp_runner (Utilities|Casting|CastToBP_Runner PossessedPawn))
  (Variables|Default|SetAs%20BP%20Runner _asbp_runner))

(fn ConstructionScript)

(fn SimulateInputwithDelay
  (Utilities|Time|SetTimerbyEvent (EventDispatchers|CreateEvent :!event Custom|SimulateInput) (Math|Random|RandomFloatinRange (Variables|Default|GetMinInputDelay) (Variables|Default|GetMaxInputDelay))))