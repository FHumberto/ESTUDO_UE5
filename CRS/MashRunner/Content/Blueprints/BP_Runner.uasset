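; Paper2D runner character for a tap-to-sprint race, driven by left/right Enhanced Input actions or NPC simulation events.
; GM_Runner's start and winner events toggle CanRun; BeginPlay also makes player 0 possess the runner.
; Taps raise MaxWalkSpeed while Tick moves it along +X and decays that speed, both scaled by velocity-based curves.
; Velocity selects the idle or run flipbook and its play rate, with footsteps played on specific frames.
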(event Custom|SimulatePowerLeft
  (if (Utilities|Enum|NotEqual(Enum) (Variables|Default|GetLastInput) "NewEnumerator2")
    (Variables|Default|SetLastInput "NewEnumerator1")
    (CallFunction|IncreaseSpeed)))

(event Custom|SimulatePowerRight
  (if (Utilities|Enum|NotEqual(Enum) (Variables|Default|GetLastInput) "NewEnumerator2")
    (Variables|Default|SetLastInput "NewEnumerator1")
    (CallFunction|IncreaseSpeed)))

(event Custom|OnAnnouncedWinner
  (Variables|Default|SetCanRun false))

(event Custom|OnStartRace
  (Variables|Default|SetCanRun true))

(event Input|EnhancedActionEvents|EnhancedInputActionIA_PowerLeft
  (params (ActionValue :type Boolean) (ElapsedSeconds :type Float%20%28double-precision%29) (TriggeredSeconds :type Float%20%28double-precision%29) (InputAction :type Input%20Action%20Object%20Reference :default "/Game/PaperAssets/Input/IA_PowerLeft.IA_PowerLeft"))
  (:Started
    (if (Utilities|Enum|NotEqual(Enum) (Variables|Default|GetLastInput) "NewEnumerator2")
      (Variables|Default|SetLastInput "NewEnumerator1")
      (CallFunction|IncreaseSpeed))))

(event Input|EnhancedActionEvents|EnhancedInputActionIA_PowerRight
  (params (ActionValue :type Boolean) (ElapsedSeconds :type Float%20%28double-precision%29) (TriggeredSeconds :type Float%20%28double-precision%29) (InputAction :type Input%20Action%20Object%20Reference :default "/Game/PaperAssets/Input/IA_PowerRight.IA_PowerRight"))
  (:Started
    (if (Utilities|Enum|NotEqual(Enum) (Variables|Default|GetLastInput) "NewEnumerator2")
      (Variables|Default|SetLastInput "NewEnumerator1")
      (CallFunction|IncreaseSpeed))))

(event EventTick
  (params (DeltaSeconds :type Float%20%28single-precision%29))
  (bind _sprite (Variables|Default|GetSprite))
  (bind _returnvalue (Class|PaperFlipbookComponent|GetPlaybackPositioninFrames _sprite))
  (Pawn|Input|AddMovementInput "1.000000,0.000000,0.000000" 1.0 false)
  (CallFunction|DecreaseSpeed DeltaSeconds)
  (CallFunction|UpdateFlipbook)
  (CallFunction|SetRunPlayrate)
  (if (== (Class|PaperFlipbookComponent|GetFlipbook (Variables|Default|GetSprite)) "/Game/PaperAssets/Runner/FB_Runner_Run.FB_Runner_Run")
    (if (or (== _returnvalue 1) (== _returnvalue 5))
      (Utilities|FlowControl|DoOnce false :!label _label
        (:Completed
          (Audio|PlaySound2D "/Game/Sounds/Footsteps/Cue_Footstep.Cue_Footstep" 1.0 1.0 0.0 0 0)))
      (else
        (goto _label Reset)))))

(event EventBeginPlay
  (Utilities|FlowControl|Sequence
    (:then_0
      (bind _asgm_runner (Utilities|Casting|CastToGM_Runner (Game|GetGameMode)))
      (Variables|Default|SetGameMode _asgm_runner)
      (EventDispatchers|BindEventtoAnnouncedWinner (Variables|Default|GetGameMode) (delegate Custom|OnAnnouncedWinner))
      (EventDispatchers|BindEventtoStartRace (Variables|Default|GetGameMode) (delegate Custom|OnStartRace)))
    (:then_1
      (Pawn|Possess (Game|GetPlayerController 0) self)
      (bind _asplayer_controller (Utilities|Casting|CastToPlayerController (Pawn|GetController)))
      (Input|AddMappingContext (PlayerController|LocalPlayerSubsystems|GetEnhancedInputLocalPlayerSubsystem _asplayer_controller) "/Game/PaperAssets/Input/IMC_Runner.IMC_Runner" 0 "(bIgnoreAllPressedKeysUntilRelease=True,bForceImmediately=False)") ; INICIALIZA OS CONTROLES
    )))

(fn ConstructionScript)

(fn IncreaseSpeed
  (bind _charactermovement (Variables|Character|GetCharacterMovement))
  (if (Variables|Default|GetCanRun)
    (Variables|/Script/Engine.CharacterMovementComponent|SetMaxWalkSpeed _charactermovement (Math|Float|Clamp(Float) (+ (Variables|/Script/Engine.CharacterMovementComponent|GetMaxWalkSpeed _charactermovement) (* (Variables|Default|GetSpeedIncreasePerTap) (Math|Curves|GetFloatValue (Variables|Default|GetSpeedIncreaseRamp) (Math|Vector|VectorLength (Variables|/Script/Engine.MovementComponent|GetVelocity (Variables|Character|GetCharacterMovement)))))) 0.0 (Variables|Default|GetMaxSpeed)))))

(fn DecreaseSpeed
  (params (DeltaSeconds :type Float%20%28double-precision%29))
  (bind _charactermovement (Variables|Character|GetCharacterMovement))
  (Variables|/Script/Engine.CharacterMovementComponent|SetMaxWalkSpeed _charactermovement (Math|Float|Max(Float) (- (Variables|/Script/Engine.CharacterMovementComponent|GetMaxWalkSpeed _charactermovement) (* DeltaSeconds (* (select (Variables|Default|GetCanRun) (Variables|Default|GetSlowMultiplier) (Variables|Default|GetSlowMujltiplierFinished)) (Math|Curves|GetFloatValue (Variables|Default|GetSpeedDecreaseRamp) (Math|Vector|VectorLength (Variables|/Script/Engine.MovementComponent|GetVelocity (Variables|Character|GetCharacterMovement))))))) 0.0)))

(fn SetRunPlayrate
  (if (== (Class|PaperFlipbookComponent|GetFlipbook (Variables|Default|GetSprite)) "/Game/PaperAssets/Runner/FB_Runner_Run.FB_Runner_Run")
    (Components|Timeline|SetPlayRate (Variables|Default|GetSprite) (/ (Math|Vector|VectorLength (Variables|/Script/Engine.MovementComponent|GetVelocity (Variables|Character|GetCharacterMovement))) (Variables|Default|GetMaxSpeed)))
    (else
      (Components|Timeline|SetPlayRate (Variables|Default|GetSprite) 1.0))))

(fn UpdateFlipbook
  (Sprite|SetFlipbook (Variables|Default|GetSprite) (select (> (Math|Vector|VectorLength (Variables|/Script/Engine.MovementComponent|GetVelocity (Variables|Character|GetCharacterMovement))) 0.0) "/Game/PaperAssets/Runner/FB_Runner_Run.FB_Runner_Run" "/Game/PaperAssets/Runner/FB_Runner_Idle.FB_Runner_Idle")))