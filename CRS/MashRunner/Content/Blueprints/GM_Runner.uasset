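; GM_Runner is the game mode for a race, handling the start signal, winner announcement and level restart.
; After a short delay on BeginPlay, it prints a start message and calls the StartRace dispatcher.
; AnnounceWinner uses IsRaceOver to accept only the first winner, prints it, calls AnnouncedWinner and sets a one-shot timer intended to delay the restart.
; RestartLevel reopens the current level by name.
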(event EventBeginPlay
  (Utilities|FlowControl|Delay 3.0)
  (Development|PrintString "RACE START")
  (Default|CallStartRace))

(fn ConstructionScript)

(fn AnnounceWinner
  (params (WinnerIndex :type Integer))
  (if (not (Variables|Default|GetIsRaceOver))
    (Variables|Default|SetIsRaceOver true)
    (Development|PrintString (Utilities|String|Append "Player " (Utilities|String|ToString(Integer) WinnerIndex) "is the winner"))
    (Default|CallAnnouncedWinner)
    (Utilities|Time|SetTimerbyEvent (EventDispatchers|CreateEvent :!event RestartLevel) 5.0) ; Adiciona Delay antes de reiniciar o level
  ))

(fn RestartLevel
  (bind _returnvalue (Game|GetCurrentLevelName true))
  (Game|OpenLevel(byName) (Utilities|String|StringToName _returnvalue)))